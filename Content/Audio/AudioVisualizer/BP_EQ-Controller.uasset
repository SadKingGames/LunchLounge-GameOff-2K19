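; Audio visualizer controller actor that drives a row of cube bars from the frequency spectrum of a selectable music track.
; On BeginPlay it sets a default track and spawns a line of BP_visCube actors along X.
; Each tick it calculates the track's spectrum at game time, one band per cube, and scales each cube's Y by its magnitude.
; A TrackNumber event switches which track is analysed; playback is not handled here.
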(event Custom|TrackNumber
  (params (TrackNumber :type Integer))
  (switch int TrackNumber
    (:0
      (Variables|Default|SetTrack "/Game/Audio/Music/Music-V2/Dissent.Dissent"))
    (:1
      (Variables|Default|SetTrack "/Game/Audio/Music/Music-V2/Sturgeon_s+Law.Sturgeon_s+Law"))
    (:2
      (Variables|Default|SetTrack "/Game/Audio/Music/Music-V2/Inner+Nuances+Fosters+Journeys.Inner+Nuances+Fosters+Journeys"))
    (:3
      (Variables|Default|SetTrack "/Game/Audio/Music/Music-V2/Eigengrau.Eigengrau"))
    (:4
      (Variables|Default|SetTrack "/Game/Audio/Music/Music-V2/In+Every+Direction.In+Every+Direction"))
    (:5
      (Variables|Default|SetTrack "/Game/Audio/Music/Music-V2/Authenticity.Authenticity"))))

(event EventBeginPlay
  (Variables|Default|SetTrack "/Game/Audio/Music/Music-V2/Dissent.Dissent")
  (CallFunction|SpawnVisualizer))

(event Collision|EventActorBeginOverlap
  (params (OtherActor :type Actor%20Object%20Reference)))

(event EventTick
  (params (DeltaSeconds :type Float%20%28single-precision%29))
  (bind _outspectrum (Class|SoundVisualizationStatics|CalculateFrequencySpectrum (Variables|Default|GetTrack) 0 (Utilities|Time|GetGameTimeinSeconds) 0.1 (Utilities|Array|Length (Variables|Default|GetBP_CubeAray))))
  (Variables|Default|SetSpectrum _outspectrum)
  (for (_array_element _array_index) (Variables|Default|GetBP_CubeAray)
    (Transformation|SetActorScale3D _array_element (Math|Vector|MakeVector 1.0 (* (Math|Float|Absolute(Float) (Utilities|Array|Get(acopy) (Variables|Default|GetSpectrum) _array_index)) 0.1) 1.0))))

(fn ConstructionScript)

(fn SpawnVisualizer
  (for _index (range 0 (- (Variables|Default|GetNumber%20of%20cubes) 1))
    (bind _returnvalue (Game|SpawnActorfromClass "/Game/Audio/AudioVisualizer/BP_visCube.BP_visCube_C" (Math|Transform|MakeTransform (+ (Transformation|GetActorLocation) (Math|Vector|MakeVector (* (Variables|Default|GetRow) (Variables|Default|GetDistance)) 1.0 0.0)) "0, 0, 0" "1,1,1") "AlwaysSpawn" 0 0))
    (Utilities|Array|Add (Variables|Default|GetBP_CubeAray) _returnvalue)
    (Math|Integer|IncrementInt (Variables|Default|GetRow))))