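; A moving obstacle Blueprint that shuttles back and forth along a spline path and can optionally damage the player on hit.
; The spline detaches at BeginPlay to stay fixed in the world, while Tick steps the actor by a per-frame speed, not scaled by delta time, reversing at each end.
; Hitting the third-person character restores its default gravity and mass and ends hanging.
; The construction script assigns the configurable mesh.
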(event Collision|EventHit
  (params (MyComp :type Primitive%20Component%20Object%20Reference) (Other :type Actor%20Object%20Reference) (OtherComp :type Primitive%20Component%20Object%20Reference) (bSelfMoved :type Boolean) (HitLocation :type Vector :default "0, 0, 0") (HitNormal :type Vector :default "0, 0, 0") (NormalImpulse :type Vector :default "0, 0, 0") (Hit :type Hit%20Result%20Structure%20%28by%20ref%29))
  (bind _asthird_person_character (Utilities|Casting|CastToThirdPersonCharacter Other))
  (Variables|/Script/Engine.CharacterMovementComponent|SetGravityScale (Variables|/Script/Engine.Character|GetCharacterMovement _asthird_person_character) (Variables|/Game/WarpPrototype/Blueprints/ThirdPersonCharacter.ThirdPersonCharacter_C|GetDefaultGravity _asthird_person_character))
  (Variables|/Script/Engine.CharacterMovementComponent|SetMass (Variables|/Script/Engine.Character|GetCharacterMovement _asthird_person_character) (Variables|/Game/WarpPrototype/Blueprints/ThirdPersonCharacter.ThirdPersonCharacter_C|GetDefaultMass _asthird_person_character))
  (Variables|/Game/WarpPrototype/Blueprints/ThirdPersonCharacter.ThirdPersonCharacter_C|SetIsHanging _asthird_person_character false)
  (if (Variables|Default|GetCanDamagePlayer)
    (Default|Damage _asthird_person_character)))

(event EventBeginPlay
  (Transformation|DetachFromComponent (Variables|Default|GetSpline) "KeepWorld" "KeepWorld" "KeepWorld" true))

(event EventTick
  (params (DeltaSeconds :type Float%20%28single-precision%29))
  (if (Variables|Default|GetGoingForward)
    (Variables|Default|SetDistance (+ (Variables|Default|GetDistance) (Variables|Default|GetSpeed)))
    (Transformation|SetActorLocation (Spline|GetLocationatDistanceAlongSpline (Variables|Default|GetSpline) (Variables|Default|GetDistance) "World") false false)
    (if (>= (Variables|Default|GetDistance) (Spline|GetSplineLength (Variables|Default|GetSpline)))
      (Variables|Default|SetGoingForward false))
    (else
      (Variables|Default|SetDistance (- (Variables|Default|GetDistance) (Variables|Default|GetSpeed)))
      (Transformation|SetActorLocation (Spline|GetLocationatDistanceAlongSpline (Variables|Default|GetSpline) (Variables|Default|GetDistance) "World") false false)
      (if (<= (Variables|Default|GetDistance) 0.0)
        (Variables|Default|SetGoingForward true)))))

(fn ConstructionScript
  (Components|StaticMesh|SetStaticMesh (Variables|Default|GetStaticMesh) (Variables|Default|GetMesh)))