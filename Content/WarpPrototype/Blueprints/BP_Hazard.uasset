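; Hazard actor with a configurable mesh that damages the ThirdPersonCharacter when it hits it.
; If IsTimedHazard is set, it loops on TimeIntervals, toggling the mesh's visibility and collision off and on.
; Before each disappearance it destroys attached BP_WarpPoints, resetting the player's hanging state, pitch, roll, gravity and mass for each, without checking which point the player uses.
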(event EventBeginPlay
  (if (Variables|Default|GetIsTimedHazard)
    (Utilities|FlowControl|Delay (Variables|Default|GetTimeIntervals) :!label _label)
    (for _array_element (Actor|GetAttachedActors)
      (bind _asbp_warp_point (Utilities|Casting|CastToBP_WarpPoint _array_element))
      (bind _asthird_person_character (Utilities|Casting|CastToThirdPersonCharacter (Game|Player|GetPlayerPawn 0)))
      (Transformation|SetActorRotation _asthird_person_character (Math|Rotator|MakeRotator 0.0 0.0 (.Yaw (Math|Rotator|BreakRotator (Transformation|GetActorRotation _asthird_person_character)))))
      (Variables|/Game/WarpPrototype/Blueprints/ThirdPersonCharacter.ThirdPersonCharacter_C|SetIsHanging _asthird_person_character false)
      (Variables|/Script/Engine.CharacterMovementComponent|SetGravityScale (Variables|/Script/Engine.Character|GetCharacterMovement _asthird_person_character) (Variables|/Game/WarpPrototype/Blueprints/ThirdPersonCharacter.ThirdPersonCharacter_C|GetDefaultGravity _asthird_person_character))
      (Variables|/Script/Engine.CharacterMovementComponent|SetMass (Variables|/Script/Engine.Character|GetCharacterMovement _asthird_person_character) (Variables|/Game/WarpPrototype/Blueprints/ThirdPersonCharacter.ThirdPersonCharacter_C|GetDefaultMass _asthird_person_character))
      (Actor|DestroyActor _asbp_warp_point))
    (Collision|SetCollisionEnabled (Variables|Default|GetStaticMesh) "NoCollision")
    (Rendering|SetVisibility (Variables|Default|GetStaticMesh) false false)
    (Utilities|FlowControl|Delay (Variables|Default|GetTimeIntervals))
    (Collision|SetCollisionEnabled (Variables|Default|GetStaticMesh) "QueryAndPhysics")
    (Rendering|SetVisibility (Variables|Default|GetStaticMesh) true false)
    (goto _label)))

(event Collision|EventHit
  (params (MyComp :type Primitive%20Component%20Object%20Reference) (Other :type Actor%20Object%20Reference) (OtherComp :type Primitive%20Component%20Object%20Reference) (bSelfMoved :type Boolean) (HitLocation :type Vector :default "0, 0, 0") (HitNormal :type Vector :default "0, 0, 0") (NormalImpulse :type Vector :default "0, 0, 0") (Hit :type Hit%20Result%20Structure%20%28by%20ref%29))
  (bind _asthird_person_character (Utilities|Casting|CastToThirdPersonCharacter Other))
  (Default|Damage _asthird_person_character))

(fn ConstructionScript
  (Components|StaticMesh|SetStaticMesh (Variables|Default|GetStaticMesh) (Variables|Default|GetMesh)))