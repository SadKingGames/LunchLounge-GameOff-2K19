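; BP_RangedEnemy is a stationary ranged enemy that telegraphs shots at the player with a laser-style aiming beam.
; BeginPlay caches the player and loops timed idle and aiming phases, ending each aim by playing a gunshot and clearing the beam, with no damage applied.
; While aiming, Tick turns mesh and aim pivot toward the player at constant speed and line-traces the beam's endpoint.
; Overlap with a warping, damage-capable player explodes and destroys it.
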(event Collision|EventActorBeginOverlap
  (params (OtherActor :type Actor%20Object%20Reference))
  (bind _asthird_person_character (Utilities|Casting|CastToThirdPersonCharacter OtherActor))
  (if (and (Variables|/Game/WarpPrototype/Blueprints/ThirdPersonCharacter.ThirdPersonCharacter_C|GetIsWarping _asthird_person_character) (Variables|/Game/WarpPrototype/Blueprints/ThirdPersonCharacter.ThirdPersonCharacter_C|GetCanDamageEnemies _asthird_person_character))
    (Effects|SpawnEmitteratLocation "/Game/BaseUnrealContent/StarterContent/Particles/P_Explosion.P_Explosion" (Transformation|GetActorLocation) "0, 0, 0" "2.000000,2.000000,2.000000")
    (Actor|DestroyActor)))

(event EventBeginPlay
  (bind _beamemitter (Variables|Default|GetBeamEmitter))
  (bind _asthird_person_character (Utilities|Casting|CastToThirdPersonCharacter (Game|Player|GetPlayerPawn 0)))
  (Variables|Default|SetPlayerRef _asthird_person_character)
  (Utilities|FlowControl|Delay 3.0 :!label _label)
  (Effects|Components|ParticleSystem|SetTemplate _beamemitter "/Game/Particles/P_Beam.P_Beam")
  (Variables|Default|SetIsAiming true)
  (Utilities|FlowControl|Delay 3.0)
  (Audio|Components|Audio|Play (Variables|Default|GetSC_TempGunshot) 0.0)
  (Variables|Default|SetIsAiming false)
  (Effects|Components|ParticleSystem|SetTemplate _beamemitter 0)
  (goto _label))

(event EventTick
  (params (DeltaSeconds :type Float%20%28single-precision%29))
  (bind _returnvalue (Utilities|Time|GetWorldDeltaSeconds))
  (bind _playerref (Variables|Default|GetPlayerRef))
  (bind _aimrotation (Variables|Default|GetAimRotation))
  (bind _beamemitter (Variables|Default|GetBeamEmitter))
  (bind _returnvalue_2 (Transformation|GetWorldRotation _aimrotation))
  (bind _returnvalue_3 (Transformation|GetWorldLocation _aimrotation))
  (bind _returnvalue_4 (Transformation|GetActorLocation _playerref))
  (bind _returnvalue_5 (Math|Rotator|FindLookatRotation _returnvalue_3 _returnvalue_4))
  (bind _returnvalue_6 (Class|KismetMathLibrary|RInterptoConstant _returnvalue_2 _returnvalue_5 _returnvalue 9e+01))
  (if (Variables|Default|GetIsAiming)
    (Transformation|SetWorldRotation (Variables|Character|GetMesh) (Math|Rotator|MakeRotator 0.0 0.0 (- (.Yaw (Math|Rotator|BreakRotator _returnvalue_6)) 9e+01)) false false)
    (Transformation|SetWorldRotation (Variables|Default|GetAimRotation) _returnvalue_6 false false)
    (bind _outhit (Collision|LineTraceByChannel (Transformation|GetWorldLocation (Variables|Default|GetAimRotation)) (* (Math|Vector|GetForwardVector _returnvalue_6) 1.5e+04) "TraceTypeQuery1" false 0 "None"))
    (Class|ParticleSystemComponent|SetBeamSourcePoint _beamemitter 0 (Transformation|GetWorldLocation _beamemitter))
    (Class|ParticleSystemComponent|SetBeamTargetPoint _beamemitter 0 (.Location (Collision|BreakHitResult _outhit)))))

(fn ConstructionScript)