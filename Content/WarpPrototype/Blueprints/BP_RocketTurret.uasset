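; BP_RocketTurret is a turret actor that periodically fires homing rockets at the player in the WarpPrototype game.
; From BeginPlay it runs an endless Delay loop, testing every few seconds whether the player pawn lies within a forward cone using a dot product against a cosine threshold.
; When the test passes, it spawns a BP_HomingRocket at the RocketSpawn component, with no range or line-of-sight check.
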(event EventBeginPlay
  (Utilities|FlowControl|Delay 5.0 :!label _label)
  (if (> (Math|Vector|DotProduct (Math|Vector|Normalize (- (Transformation|GetActorLocation (Game|Player|GetPlayerPawn 0)) (Transformation|GetActorLocation))) (Transformation|GetActorForwardVector)) (Math|Trig|Cos(Degrees) 6e+01))
    (Game|SpawnActorfromClass "/Game/WarpPrototype/Blueprints/BP_HomingRocket.BP_HomingRocket_C" (Math|Conversions|ToTransform(Vector) (Transformation|GetWorldLocation (Variables|Default|GetRocketSpawn))) "Undefined" 0 0)
    (goto _label)
    (else
      (goto _label))))

(fn ConstructionScript)